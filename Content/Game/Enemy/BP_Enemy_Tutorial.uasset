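; BP_Enemy_Tutorial is an enemy variant for the tutorial, built on a parent enemy class.
; On death it runs the parent logic, then calls ProgressTutorial on its tutorial reference.
; When it enters its crouching stance after a firing sequence, it immediately restarts a randomized firing timer if firing is enabled.
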(event `self.Death`
  ;[1 1 1] Progress tutorial on the enemies death.
  (`parent.Death`)
  (`/Game/Game/Tutorial/BP_TutorialManager_Base.Progress Tutorial` (`self.TutorialRef`)))

(event `self.Crouching Stance`
  ;[1 1 1] Immediately reset firing timer on firing sequence completion
  (`parent.Crouching Stance`)
  (if (`self.Firing Enabled`)
    (`self.Set Firing Timer` 1.0)))

(fn `UserConstructionScript`
  (`parent.UserConstructionScript`))