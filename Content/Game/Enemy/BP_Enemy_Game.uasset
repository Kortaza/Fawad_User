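; Game-specific enemy Blueprint that extends a parent enemy, adding relocation between manager-assigned locations during its firing cycle.
; On returning to crouching stance, a random roll against ChanceToMove asks the enemy manager for a move, otherwise restarting a randomized firing timer.
; MoveToNewLocation uses SimpleMoveToLocation toward LocationRef, flags the enemy as moving and clears the firing sequence timer.
; Death frees the held location in the manager before running parent logic.
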(event `self.Death`
  ;[1 1 1] Special cleanup on enemy death
  (`/Game/Game/Enemy/BP_EnemyManager.FreeLocation` (`self.EnemyManagerRef`) (`self.LocationRef`))
  (`parent.Death`))

(event `self.Crouching Stance`
  ;[1 1 1] At the end of the firing sequence, check if enemy should move or reset firing sequence
  (`parent.Crouching Stance`)
  (if (<= (`KismetMathLibrary.RandomFloatInRange` 0.0 1.0) (`self.Chance to Move `))
    (bind _move_available (`/Game/Game/Enemy/BP_EnemyManager.MoveEnemy` (`self.EnemyManagerRef`) self))
    (if (not _move_available)
      (`self.Set Firing Timer` 1.0 :!label _label))
    (else
      (goto _label))))

(event `MoveToNewLocation`
  ;[1 1 1] Start movement to new location
  (`AIBlueprintHelperLibrary.SimpleMoveToLocation` (`self.GetController`) (`SceneComponent.K2_GetComponentLocation` (`self.LocationRef`)))
  (set `self.Moving` true)
  (`KismetSystemLibrary.K2_ClearTimer` null "Start Firing Sequence"))

(fn `UserConstructionScript`
  (`parent.UserConstructionScript`))