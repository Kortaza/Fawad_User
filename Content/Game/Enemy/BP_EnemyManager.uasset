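; Enemy manager that spawns BP_Enemy_Game actors at thirteen spawn points and relocates them between those points.
; Open and closed lists track free and occupied points, with GetNewLocation claiming a random free one and FreeLocation releasing it.
; StartEnemySpawning begins a self-rescheduling timer whose interval shrinks after each successful spawn, down to a floor.
; DestroyAllEnemies removes every BP_Enemy_Base actor and stops spawning; BeginPlay starts nothing.
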(event `self.ReceiveBeginPlay`)

(fn `DestroyAllEnemies`
  (`|ExecutionSequence`
    (:`then_0`
      (bind _outactors (`GameplayStatics.GetAllActorsOfClass` "/Game/Game/Enemy/BP_Enemy_Base.BP_Enemy_Base_C"))
      (for _array_element _outactors
        (`self.K2_DestroyActor` _array_element)))
    (:`then_1`
      (`KismetArrayLibrary.Array_Clear` (`self.ClosedList`))
      (`KismetSystemLibrary.K2_ClearTimer` null "SpawnEnemy"))))

(fn `FreeLocation`
  (params (LocationRef :type "CapsuleComponent Object Reference"))
  (locals (ClosedIndex :type Integer))
  (bind _returnvalue (`KismetArrayLibrary.Array_RemoveItem` (`self.ClosedList`) LocationRef))
  (if _returnvalue
    (`KismetArrayLibrary.Array_Add` (`self.OpenList`) LocationRef)))

(fn `GetNewLocation`
  (returns (Available :type Boolean) (NewLoc :type "CapsuleComponent Object Reference"))
  (locals (OpenIndex :type Integer) (SpawnRef :type "CapsuleComponent Object Reference"))
  (bind _openlist (`self.OpenList`))
  (bind _returnvalue (`KismetArrayLibrary.Array_Length` _openlist))
  (if (> _returnvalue 0)
    (set `local.OpenIndex` (`KismetMathLibrary.RandomIntegerInRange` 0 (- _returnvalue 1)))
    (set `local.SpawnRef` (`|GetArrayItem` _openlist (`local.OpenIndex`)))
    (`KismetArrayLibrary.Array_Add` (`self.ClosedList`) (`local.SpawnRef`))
    (`KismetArrayLibrary.Array_Remove` (`self.OpenList`) (`local.OpenIndex`))
    (return true (`local.SpawnRef`))
    (else
      (return false null))))

(fn `MoveEnemy`
  (params (Enemy :type "/Game/Game/Enemy/BP_Enemy_Game Object Reference"))
  (returns (`Move Available` :type Boolean))
  (locals (ClosedIndex :type Integer) (OpenIndex :type Integer) (OldSpawnRef :type "CapsuleComponent Object Reference"))
  (set `local.OldSpawnRef` (`/Game/Game/Enemy/BP_Enemy_Base.LocationRef` Enemy))
  (bind (_available _newloc) (`self.GetNewLocation`))
  (if _available
    (set `/Game/Game/Enemy/BP_Enemy_Base.LocationRef` _newloc Enemy)
    (`/Game/Game/Enemy/BP_Enemy_Game.MoveToNewLocation` Enemy)
    (`self.FreeLocation` (`local.OldSpawnRef`))
    (return true)
    (else
      (return false))))

(fn `SpawnEnemy`
  (bind (_available _newloc) (`self.GetNewLocation`))
  (if _available
    (bind _returnvalue (`|SpawnActorFromClass` "/Game/Game/Enemy/BP_Enemy_Game.BP_Enemy_Game_C" (`SceneComponent.K2_GetComponentToWorld` _newloc) "Undefined" "OverrideRootScale" null _newloc self null))
    (`/Game/Game/Enemy/BP_Enemy_Base.Set Firing Timer` _returnvalue 1.0 5.0)
    (set `self.EnemySpawnTimer` (`KismetMathLibrary.FClamp` (- (`self.EnemySpawnTimer`) 0.1) 2.0 50.0)))
  (`KismetSystemLibrary.K2_SetTimer` null "SpawnEnemy" (`self.EnemySpawnTimer`)))

(fn `StartEnemySpawning`
  (set `self.OpenList` (`|MakeArray` (`self.Spawn 00`) (`self.Spawn 01`) (`self.Spawn 02`) (`self.Spawn 03`) (`self.Spawn 04`) (`self.Spawn 05`) (`self.Spawn 06`) (`self.Spawn 07`) (`self.Spawn 08`) (`self.Spawn 09`) (`self.Spawn 10`) (`self.Spawn 11`) (`self.Spawn 12`)))
  (set `self.EnemySpawnTimer` (`self.StartingEnemySpawnTimer`))
  (`KismetSystemLibrary.K2_SetTimer` null "SpawnEnemy" (`self.EnemySpawnTimer`)))

(fn `UserConstructionScript`)