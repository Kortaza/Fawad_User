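; BP_Projectile is a shot fired by players or enemies, with speed and material set by PlayerOwned and self-destruction after a lifetime.
; Each tick it line-traces the distance it would travel, moving forward only when nothing is hit.
; Hitting a MotionControllerPawn's HitBox damages the pawn; that or any non-pawn hit destroys the projectile.
; Hits on the tutorial manager's dodged-projectile collision advance the tutorial, needing a second hit in one state.
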(event `self.ReceiveBeginPlay`
  ;[1 1 1] Setup lifetime to destroy and set speed based on player/enemy ownership
  (`KismetSystemLibrary.K2_SetTimerDelegate` (delegate `Destroy Self`) (`self.Lifetime`))
  (if (`self.PlayerOwned`)
    (set `self.Speed` 20000.0)
    (`PrimitiveComponent.SetMaterial` (`self.Sphere`) 0 "/Game/Game/Player/Materials/MI_ProjectilePlayer.MI_ProjectilePlayer")
    (else
      (set `self.Speed` 1500.0)
      (`PrimitiveComponent.SetMaterial` (`self.Sphere`) 0 "/Game/Game/Player/Materials/MI_ProjectileEnemy.MI_ProjectileEnemy"))))

(event `Destroy Self`
  ;[1 1 1] Setup lifetime to destroy and set speed based on player/enemy ownership
  (`self.K2_DestroyActor`))

(event `self.ReceiveTick`
  (params (DeltaSeconds :type "Float (single-precision)"))
  (bind _returnvalue (`SceneComponent.K2_GetComponentLocation` (`self.Origin`)))
  (bind _returnvalue_2 (+ _returnvalue (* (`SceneComponent.GetForwardVector` (`self.Origin`)) (* DeltaSeconds (`self.Speed`)))))
  ;[1 1 1] Movement based on speed and ray tracing
  (bind (_outhit _returnvalue_3) (`KismetSystemLibrary.LineTraceSingle` _returnvalue _returnvalue_2 "TraceTypeQuery4"))
  (if _returnvalue_3
    (bind (_bblockinghit _binitialoverlap _time _distance _location _impactpoint _normal _impactnormal _physmat _hitactor _hitcomponent) (`GameplayStatics.BreakHitResult` _outhit))
    (bind _asmotion_controller_pawn (cast `/Game/Game/Player/MotionControllerPawn` _hitactor)
      (:`then`
        (if (== (`/Game/Game/Player/MotionControllerPawn.HitBox` _asmotion_controller_pawn) _hitcomponent)
          (`/Game/Game/Player/MotionControllerPawn.Damage` _asmotion_controller_pawn)
          (`self.Destroy Self`)))
      (:`CastFailed`
        ;[1 1 1] Tutorial section for dodged projectile
        (bind _asbp_tutorial_manager_base (cast `/Game/Game/Tutorial/BP_TutorialManager_Base` _hitactor)
          (:`then`
            (if (== (`/Game/Game/Tutorial/BP_TutorialManager_Base.Dodged Projectile Collision` _asbp_tutorial_manager_base) _hitcomponent)
              (bind _asbp_tutorial_manager_user (cast `/Game/Game/Tutorial/BP_TutorialManager_User` _asbp_tutorial_manager_base)
                (:`then`
                  (if (`|EnumEquality` (`/Game/Game/Tutorial/BP_TutorialManager_User.TutorialState` _asbp_tutorial_manager_user) "NewEnumerator19")
                    (if (`/Game/Game/Tutorial/BP_TutorialManager_User.FirstShotHit` _asbp_tutorial_manager_user)
                      (`/Game/Game/Tutorial/BP_TutorialManager_Base.Progress Tutorial` _asbp_tutorial_manager_base :!label _label)
                      (else
                        (set `/Game/Game/Tutorial/BP_TutorialManager_User.FirstShotHit` true _asbp_tutorial_manager_user)))
                    (else
                      (goto _label))))
                (:`CastFailed`
                  (goto _label)))
              (`self.Destroy Self`)
              (else
                (`self.Destroy Self` :!label _label_2))))
          (:`CastFailed`
            (goto _label_2)))))
    (else
      (`SceneComponent.K2_SetWorldLocation` (`self.DefaultSceneRoot`) _returnvalue_2 false false)
      (`SceneComponent.K2_SetWorldLocation` (`self.Origin`) _returnvalue_2 false false))))

(fn `UserConstructionScript`)