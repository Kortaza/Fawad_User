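; Base enemy that crouches, stands to aim and shoots projectiles at the MotionControllerPawn player's hit box.
; A random timer starts the stance cycle, while Tick ramps aim percentage to switch stances and yaws the body toward the player when stationary.
; Reaching a move target snaps it into place and restarts the timer.
; Hits flash a dynamic material and reduce health to a death stance; Shatter spawns a shatter actor, credits the kill and destroys the enemy.
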(event `self.ReceiveBeginPlay`
  (`|ExecutionSequence`
    (:`then_0`
      ;[1 1 1] Setup socket attachments for weapon and projectile spawn
      (`SceneComponent.K2_AttachToComponent` (`self.Weapon`) (`self.Mesh`) "Socket_Weapon" "SnapToTarget" "SnapToTarget" "SnapToTarget" true)
      (`SceneComponent.K2_AttachToComponent` (`self.Projectile Spawn`) (`self.Mesh`) "Socket_ProjectileSpawn" "SnapToTarget" "SnapToTarget" "SnapToTarget" true))
    (:`then_1`
      ;[1 1 1] Upload variables to the Animation Blueprint
      (bind _asanim_bp_enemy (cast `/Game/AnimStarterPack/AnimBP_Enemy` (`SkeletalMeshComponent.GetAnimInstance` (`self.Mesh`))))
      (set `/Game/AnimStarterPack/AnimBP_Enemy.BurstFireNumber` (`self.BurstFireCount`) _asanim_bp_enemy))
    (:`then_2`
      ;[1 1 1] Getting and storing player reference
      (bind _outactors (`GameplayStatics.GetAllActorsOfClass` "/Game/Game/Player/MotionControllerPawn.MotionControllerPawn_C"))
      (for _array_element _outactors
        (set `self.PlayerRef` _array_element)))
    (:`then_3`
      (bind _returnvalue (`KismetMaterialLibrary.CreateDynamicMaterialInstance` "/Game/AnimStarterPack/UE4_Mannequin/Materials/MI_Enemy.MI_Enemy"))
      (set `self.Material_Body` _returnvalue)
      (`PrimitiveComponent.SetMaterial` (`self.Mesh`) 0 (`self.Material_Body`))
      (`MaterialInstanceDynamic.SetVectorParameterValue` (`self.Material_Body`) "BodyColor" (`self.DefaultColor`)))))

(event `Set Firing Timer`
  (params (`Minimum Time to Fire` :type "Float (double-precision)" :default 1.0) (`Maximum Time to Fire` :type "Float (double-precision)" :default 5.0))
  ;[1 1 1] Idle/Firing stance switching
  (bind _output_get (set `self.DelayBetweenFiring` (`KismetMathLibrary.RandomFloatInRange` `Minimum Time to Fire` `Maximum Time to Fire`)))
  (`KismetSystemLibrary.K2_SetTimer` null "Start Firing Sequence" _output_get))

(event `Standing Up Stance`
  ;[1 1 1] Idle/Firing stance switching
  (set `self.Stance` "NewEnumerator1"))

(event `Aim Stance`
  ;[1 1 1] Idle/Firing stance switching
  (set `self.Stance` "NewEnumerator2"))

(event `Fire Stance`
  ;[1 1 1] Idle/Firing stance switching
  (set `self.Stance` "NewEnumerator3"))

(event `Stop Aim Stance`
  ;[1 1 1] Idle/Firing stance switching
  (set `self.Stance` "NewEnumerator4"))

(event `Crouch Down Stance`
  ;[1 1 1] Idle/Firing stance switching
  (set `self.Stance` "NewEnumerator5"))

(event `Crouching Stance`
  ;[1 1 1] Idle/Firing stance switching
  (set `self.Stance` "NewEnumerator0"))

(event `self.ReceiveTick`
  (params (DeltaSeconds :type "Float (single-precision)"))
  (bind _deltatick (`self.DeltaTick`))
  (bind (_returnvalue_roll _returnvalue_pitch _returnvalue_yaw) (`KismetMathLibrary.BreakRotator` (`KismetMathLibrary.FindLookAtRotation` (`SceneComponent.K2_GetComponentLocation` (`self.CapsuleComponent`)) (`SceneComponent.K2_GetComponentLocation` (`/Game/Game/Player/MotionControllerPawn.HitBox` (`self.PlayerRef`))))))
  (set `self.DeltaTick` DeltaSeconds)
  (`|ExecutionSequence`
    (:`then_0`
      ;[1 1 1] Update aiming percentage using delta tick when in the aiming stances
      (switch `/Game/Game/Enemy/EnemyStance` (`self.Stance`)
        (:`NewEnumerator2`
          (bind _output_get (set `self.AimPercentage` (`KismetMathLibrary.FClamp` (+ (`self.AimPercentage`) (* (`self.AimRate`) (`self.DeltaTick`))))))
          (if (>= _output_get 0.97)
            (`self.Fire Stance`)))
        (:`NewEnumerator4`
          (bind _output_get_2 (set `self.AimPercentage` (`KismetMathLibrary.FClamp` (- (`self.AimPercentage`) (* (`self.AimDropRate`) (`self.DeltaTick`))))))
          (if (<= _output_get_2 0.03)
            (`self.Crouch Down Stance`)))))
    (:`then_1`
      (if (`self.Moving`)
        ;[1 1 1] Movement complete - Start firing timer again
        (if (`PrimitiveComponent.IsOverlappingComponent` (`self.LocationRef`) (`self.CenterPoint`))
          (set `self.Moving` false)
          (`SceneComponent.K2_SetWorldLocation` (`self.CapsuleComponent`) (`SceneComponent.K2_GetComponentLocation` (`self.LocationRef`)) false false)
          (`self.Set Firing Timer` 1.0))
        (else
          ;[1 1 1] Set rotation to always be looking at the player
          (`SceneComponent.K2_SetWorldRotation` (`self.CapsuleComponent`) (`KismetMathLibrary.MakeRotator` 0.0 0.0 _returnvalue_yaw) false false))))
    (:`then_2`
      ;[1 1 1] Changing Body color on hits to indicate damage
      (if (`self.HitMarked`)
        (set `self.HitMarkedLerp` (`KismetMathLibrary.FClamp` (+ (* _deltatick 5.0) (`self.HitMarkedLerp`))))
        (else
          (set `self.HitMarkedLerp` (`KismetMathLibrary.FClamp` (- (`self.HitMarkedLerp`) (* _deltatick 2.0))))))
      (`MaterialInstanceDynamic.SetVectorParameterValue` (`self.Material_Body`) "BodyColor" (`KismetMathLibrary.LinearColorLerp` (`self.DefaultColor`) (`self.HitColor`) (`self.HitMarkedLerp`)))
      (if (and (>= (`self.HitMarkedLerp`) 0.99) (> (`self.Health`) 0))
        (set `self.HitMarked` false)))))

(event `Damage`
  (bind _health (`self.Health`))
  ;[1 1 1] Take damage and kill if necessary
  (set `self.HitMarked` true)
  (`/Engine/EditorBlueprintResources/StandardMacros.DecrementInt` _health
    (:`  `
      (if (<= _health 0)
        (set `self.Stance` "NewEnumerator6")
        (`NavMovementComponent.StopActiveMovement` (`self.CharacterMovement`))))))

(event `Death`
  ;[1 1 1] Destroy Actor on Death
  (`/Engine/EditorBlueprintResources/StandardMacros.IncrementInt` (`/Game/Game/Player/MotionControllerPawn.Kills` (`self.PlayerRef`))))

(event `Shatter`
  (`|SpawnActorFromClass` "/Game/Game/Enemy/BP_EnemyShatter.BP_EnemyShatter_C" (`SceneComponent.K2_GetComponentToWorld` (`self.Mesh`)) "AlwaysSpawn" "OverrideRootScale" null null)
  (`self.Death`)
  (`self.K2_DestroyActor`))

(fn `Fire`
  (bind _returnvalue (`|SpawnActorFromClass` "/Game/Game/Enemy/BP_Projectile.BP_Projectile_C" (`SceneComponent.K2_GetComponentToWorld` (`self.Projectile Spawn`)) "Undefined" "OverrideRootScale" null false null))
  (`SceneComponent.K2_SetWorldRotation` (`/Game/Game/Enemy/BP_Projectile.Origin` _returnvalue) (`KismetMathLibrary.FindLookAtRotation` (`SceneComponent.K2_GetComponentLocation` (`/Game/Game/Enemy/BP_Projectile.Origin` _returnvalue)) (`SceneComponent.K2_GetComponentLocation` (`/Game/Game/Player/MotionControllerPawn.HitBox` (`self.PlayerRef`)))) false false))

(fn `Start Firing Sequence`
  (`self.Standing Up Stance`)
  (set `self.Firing Enabled` true))

(fn `Stop Firing`
  (`KismetSystemLibrary.K2_ClearTimer` null "Start Firing Sequence")
  (set `self.Firing Enabled` false))

(fn `UserConstructionScript`)