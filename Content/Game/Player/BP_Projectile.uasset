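; BP_Projectile is a shot fired by the player or an enemy, with ownership setting its speed and material and a timer limiting its lifetime.
; Each Tick it line-traces along the coming frame's travel instead of using collision sweeps, moving forward only when nothing blocks.
; Player shots damage ThirdPersonCharacter, while enemy shots damage MotionControllerPawn only through its HitBox.
; Blocking hits destroy it, except enemy shots striking other pawn components, which stall.
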(event `self.ReceiveBeginPlay`
  ;[1 1 1] Setup lifetime to destroy and set speed based on player/enemy ownership
  (`KismetSystemLibrary.K2_SetTimerDelegate` (delegate `Destroy Self`) (`self.Lifetime`))
  (if (`self.PlayerOwned`)
    (set `self.Speed` 30000.0)
    (`PrimitiveComponent.SetMaterial` (`self.Sphere`) 0 "/Game/Game/Player/Materials/MI_ProjectilePlayer.MI_ProjectilePlayer")
    (else
      (set `self.Speed` 1500.0)
      (`PrimitiveComponent.SetMaterial` (`self.Sphere`) 0 "/Game/Game/Player/Materials/MI_ProjectileEnemy.MI_ProjectileEnemy"))))

(event `Destroy Self`
  ;[1 1 1] Setup lifetime to destroy and set speed based on player/enemy ownership
  (`self.K2_DestroyActor`))

(event `self.ReceiveTick`
  (params (DeltaSeconds :type "Float (single-precision)"))
  (bind _returnvalue (`SceneComponent.K2_GetComponentLocation` (`self.Origin`)))
  (bind _returnvalue_2 (+ _returnvalue (* (`SceneComponent.GetForwardVector` (`self.Origin`)) (* DeltaSeconds (`self.Speed`)))))
  ;[1 1 1] Movement based on speed and ray tracing
  (bind (_outhit _returnvalue_3) (`KismetSystemLibrary.LineTraceSingle` _returnvalue _returnvalue_2 "TraceTypeQuery1"))
  (if _returnvalue_3
    (if (`self.PlayerOwned`)
      (bind (_bblockinghit _binitialoverlap _time _distance _location _impactpoint _normal _impactnormal _physmat _hitactor _hitcomponent) (`GameplayStatics.BreakHitResult` _outhit))
      (bind _asthird_person_character (cast `/Game/Game/ThirdPersonCharacter` _hitactor)
        (:`then`
          (`/Game/Game/ThirdPersonCharacter.Damage` _asthird_person_character))
        (:`CastFailed`
          _))
      (`self.Destroy Self`)
      (else
        (bind _asmotion_controller_pawn (cast `/Game/Game/Player/MotionControllerPawn` _hitactor)
          (:`then`
            (if (== (`/Game/Game/Player/MotionControllerPawn.HitBox` _asmotion_controller_pawn) _hitcomponent)
              (`/Game/Game/Player/MotionControllerPawn.Damage` _asmotion_controller_pawn)
              (`self.Destroy Self` :!label _label)))
          (:`CastFailed`
            (goto _label)))))
    (else
      (`SceneComponent.K2_SetWorldLocation` (`self.DefaultSceneRoot`) _returnvalue_2 false false)
      (`SceneComponent.K2_SetWorldLocation` (`self.Origin`) _returnvalue_2 false false))))

(fn `UserConstructionScript`)