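; Player laser beam visual that appears between a weapon location and a target location, then fades out.
; On BeginPlay it centers the scene component between both points, scales its Z by their distance and aims it at the target.
; Tick lowers a dynamic material's opacity and the X/Y scale using FadeLerp, destroying the actor at 99, long after the fade reaches zero at 1.
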(event `self.ReceiveBeginPlay`
  (bind _weaponloc (`self.WeaponLoc`))
  (bind _targetloc (`self.TargetLoc`))
  (bind (_returnvalue_x _returnvalue_y) (`KismetMathLibrary.BreakVector` (`SceneComponent.K2_GetComponentScale` (`self.Scene`))))
  (`SceneComponent.K2_SetWorldLocation` (`self.Scene`) (* (+ _targetloc _weaponloc) 0.5) false false)
  (`SceneComponent.SetWorldScale3D` (`self.Scene`) (`KismetMathLibrary.MakeVector` _returnvalue_x _returnvalue_y (* (`KismetMathLibrary.VSize` (- _targetloc _weaponloc)) 0.01)))
  (`SceneComponent.K2_SetWorldRotation` (`self.Scene`) (`KismetMathLibrary.FindLookAtRotation` (`self.WeaponLoc`) (`self.TargetLoc`)) false false))

(event `self.ReceiveTick`
  (params (DeltaSeconds :type "Float (single-precision)"))
  (bind (_returnvalue_x _returnvalue_y _returnvalue_z) (`KismetMathLibrary.BreakVector` (`SceneComponent.K2_GetComponentScale` (`self.Scene`))))
  (bind _output_get (set `self.FadeLerp` (+ (`self.FadeLerp`) (* DeltaSeconds 10.0))))
  (bind _returnvalue (`KismetMathLibrary.Lerp` 1.0 0.0 _output_get))
  (`MaterialInstanceDynamic.SetScalarParameterValue` (`self.Material`) "Opacity" _returnvalue)
  (`SceneComponent.SetWorldScale3D` (`self.Scene`) (`KismetMathLibrary.MakeVector` _returnvalue _returnvalue _returnvalue_z))
  (if (>= (`self.FadeLerp`) 99.0)
    (`self.K2_DestroyActor`)))

(fn `UserConstructionScript`
  (bind _returnvalue (`KismetMaterialLibrary.CreateDynamicMaterialInstance` "/Game/Game/Player/Materials/MI_ProjectilePlayer.MI_ProjectilePlayer"))
  (set `self.Material` _returnvalue)
  (`PrimitiveComponent.SetMaterial` (`self.Sphere`) 0 (`self.Material`)))