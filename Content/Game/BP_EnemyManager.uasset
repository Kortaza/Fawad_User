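; BP_EnemyManager spawns enemy ThirdPersonCharacters at a fixed set of spawn points and manages which points are occupied.
; A looping timer calls SpawnEnemy, which takes a random free point from OpenList, moves it to ClosedList and passes it to the new enemy with a manager reference.
; MoveEnemy relocates an enemy to another free point and returns its old one through FreeLocation.
; Spawning and moving do nothing when no point is free.
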(event `self.ReceiveBeginPlay`
  (set `self.OpenList` (`|MakeArray` (`self.Spawn 00`) (`self.Spawn 01`) (`self.Spawn 02`) (`self.Spawn 03`) (`self.Spawn 04`) (`self.Spawn 05`) (`self.Spawn 06`) (`self.Spawn 07`) (`self.Spawn 08`) (`self.Spawn 09`) (`self.Spawn 10`) (`self.Spawn 11`) (`self.Spawn 12`)))
  (`KismetSystemLibrary.K2_SetTimer` null "SpawnEnemy" (`self.EnemySpawnTimer`) true))

(fn `FreeLocation`
  (params (LocationRef :type "CapsuleComponent Object Reference"))
  (locals (ClosedIndex :type Integer))
  (bind _returnvalue (`KismetArrayLibrary.Array_RemoveItem` (`self.ClosedList`) LocationRef))
  (if _returnvalue
    (`KismetArrayLibrary.Array_Add` (`self.OpenList`) LocationRef)))

(fn `GetNewLocation`
  (returns (Available :type Boolean) (NewLoc :type "CapsuleComponent Object Reference"))
  (locals (OpenIndex :type Integer) (SpawnRef :type "CapsuleComponent Object Reference"))
  (bind _openlist (`self.OpenList`))
  (bind _returnvalue (`KismetArrayLibrary.Array_Length` _openlist))
  (if (> _returnvalue 0)
    (set `local.OpenIndex` (`KismetMathLibrary.RandomIntegerInRange` 0 (- _returnvalue 1)))
    (set `local.SpawnRef` (`|GetArrayItem` _openlist (`local.OpenIndex`)))
    (`KismetArrayLibrary.Array_Add` (`self.ClosedList`) (`local.SpawnRef`))
    (`KismetArrayLibrary.Array_Remove` (`self.OpenList`) (`local.OpenIndex`))
    (return true (`local.SpawnRef`))
    (else
      (return false null))))

(fn `MoveEnemy`
  (params (Enemy :type "/Game/Game/ThirdPersonCharacter Object Reference"))
  (locals (ClosedIndex :type Integer) (OpenIndex :type Integer) (OldSpawnRef :type "CapsuleComponent Object Reference"))
  (set `local.OldSpawnRef` (`/Game/Game/ThirdPersonCharacter.LocationRef` Enemy))
  (bind (_available _newloc) (`self.GetNewLocation`))
  (if _available
    (set `/Game/Game/ThirdPersonCharacter.LocationRef` _newloc Enemy)
    (`/Game/Game/ThirdPersonCharacter.MoveToNewLocation` Enemy)
    (`self.FreeLocation` (`local.OldSpawnRef`))))

(fn `SpawnEnemy`
  (bind (_available _newloc) (`self.GetNewLocation`))
  (if _available
    (`|SpawnActorFromClass` "/Game/Game/ThirdPersonCharacter.ThirdPersonCharacter_C" (`SceneComponent.K2_GetComponentToWorld` _newloc) "Undefined" "OverrideRootScale" null _newloc self null)))

(fn `UserConstructionScript`)